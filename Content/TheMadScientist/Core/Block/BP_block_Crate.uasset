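; BP_block_Crate is a destructible crate block that breaks after taking projectile hits.
; Each TakeDamage event removes one health point; at zero it spawns a Niagara explosion at its location and destroys itself.
; When health drops to the crack threshold, a DoOnce swaps its texture to a cracked version a single time.
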(event EventTakeDamage
  ;[1 1 1] Gère la prise lorsque l'on est touché par un projectile
  (bind _result (Math|Integer|DecrementInt (Variables|Default|GetHealthPoints)) ; retire un pv à chaque fois\nqu'un projectile touche\nla caisse
    (:%20%20
      (if (<= _result 0) ; Si on n'as plus de PV
        (Niagara|SpawnSystematLocation "/Game/TheMadScientist/Core/Niagara_System/NS_Explosion.NS_Explosion" (Transformation|GetActorLocation))
        (Actor|DestroyActor)
        (elif (<= _result (Variables|Default|GetCrackTreshold))
          (Utilities|FlowControl|DoOnce false
            (:Completed
              (CallFunction|UpdateTexture "/Game/TheMadScientist/Art/Interactables/Crate/T_Crate_Cracked.T_Crate_Cracked"))))))))

(fn ConstructionScript
  (|CallParentFunction))