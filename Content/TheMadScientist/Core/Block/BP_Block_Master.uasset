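; BP_Block_Master is a block Blueprint, apparently the base for block actors, that sets up the look of its Cube mesh.
; The construction script passes the Texture variable to UpdateTexture, so the look is applied at construction.
; UpdateTexture creates a dynamic material instance on the Cube, sets its texture, and feeds the front, back, left and right visibility variables in as scalar parameters.
; The event graph holds no active logic.
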(event EventBeginPlay)

(event Collision|EventActorBeginOverlap
  (params (OtherActor :type Actor%20Object%20Reference)))

(event EventTick
  (params (DeltaSeconds :type Float%20%28single-precision%29)))

(fn ConstructionScript
  (CallFunction|UpdateTexture (Variables|Default|GetTexture)))

(fn UpdateTexture
  (params (NewTexture :type Texture%20Object%20Reference))
  (bind _returnvalue (Rendering|Material|CreateDynamicMaterialInstance (Variables|Components|GetCube) 0 0 "None" :!class /Script/Engine.PrimitiveComponent))
  (Rendering|Material|SetTextureParameterValue _returnvalue "Texture" NewTexture)
  (Rendering|Material|SetScalarParameterValue _returnvalue "Show Front" (Math|Conversions|ToFloat(Boolean) (Variables|Default|GetShowFront)) :!class /Script/Engine.MaterialInstanceDynamic)
  (Rendering|Material|SetScalarParameterValue _returnvalue "Show Back" (Math|Conversions|ToFloat(Boolean) (Variables|Default|GetShowBack)) :!class /Script/Engine.MaterialInstanceDynamic)
  (Rendering|Material|SetScalarParameterValue _returnvalue "Show Left" (Math|Conversions|ToFloat(Boolean) (Variables|Default|GetShowLeft)) :!class /Script/Engine.MaterialInstanceDynamic)
  (Rendering|Material|SetScalarParameterValue _returnvalue "Show Right" (Math|Conversions|ToFloat(Boolean) (Variables|Default|GetShowRight)) :!class /Script/Engine.MaterialInstanceDynamic))