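; BP_Enemy1 is a patrolling enemy that damages what it bumps into and can be killed.
; Two custom events chain AIMoveTo calls to shuttle it between Point1 and Point2, continuing only on successful moves.
; Capsule hits send a damage message to the other actor, while its own TakeDamage decrements HealthPoints, then spawns a Niagara explosion and destroys it at zero.
; An older timeline-driven patrol using TurnChar remains disconnected.
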(event OnComponentHit(CapsuleComponent)
  (params (HitComponent :type Primitive%20Component%20Object%20Reference) (OtherActor :type Actor%20Object%20Reference) (OtherComp :type Primitive%20Component%20Object%20Reference) (NormalImpulse :type Vector :default "0, 0, 0") (Hit :type Hit%20Result%20Structure%20%28by%20ref%29))
  (Class|BPIDamageable|TakeDamage(Message) OtherActor))

(event Custom|ExecA
  ;[1 1 1] Permet à l'enemy de se dépacler d'un point A vers un point B
  (AI|AIMoveTo self (Variables|Default|GetPoint1) 0 5.0 false
    (:OnSuccess
      (CallFunction|ExecB))))

(event Custom|ExecB
  ;[1 1 1] Permet à l'enemy de se dépacler d'un point A vers un point B
  (AI|AIMoveTo self (Variables|Default|GetPoint2) 0 5.0 false
    (:OnSuccess
      (CallFunction|ExecA))))

(event EventBeginPlay
  ;[1 1 1] Permet à l'enemy de se dépacler d'un point A vers un point B
  (CallFunction|ExecA))

(event EventTakeDamage
  ;[1 1 1] Gère la prise lorsque l'on est touché par un projectile
  (bind _result (Math|Integer|DecrementInt (Variables|Default|GetHealthPoints))
    (:%20%20
      (if (<= _result 0) ; Si on n'as plus de PV
        (Niagara|SpawnSystematLocation "/Game/TheMadScientist/Core/Niagara_System/NS_Explosion.NS_Explosion" (Transformation|GetActorLocation))
        (Actor|DestroyActor)))))

(fn ConstructionScript)

(fn TurnChar
  (Transformation|SetActorRotation (Math|Rotator|CombineRotators (Transformation|GetActorRotation) "0.000000,180.000000,0.000000")))